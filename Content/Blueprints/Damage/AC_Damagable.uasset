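; Actor component that gives its owner health, damage intake and healing.
; TakeDamage uses a Should Damage check on death, invincibility and blocking to branch into block, damage or no damage, with per-hit overrides from DamageInfo.
; Damage lowers clamped health, then raises death or, if interruptible or forced, a damage response.
; Healing adds a fraction of max health, and both health changes broadcast an update.
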(fn TakeDamage
  (params (Damage%20Info :type S%20Damage%20Info%20Structure) (Damage%20Causer :type Actor%20Object%20Reference))
  (bind (_amount _shoulddamageinvinciable _canbeblocked_) (Utilities|Struct|BreakS_DamageInfo Damage%20Info))
  (bind (_damageresponse _shouldforceinturrupt) (Utilities|Struct|BreakS_DamageInfo Damage%20Info))
  (Utilities|ShouldDamage? _shoulddamageinvinciable _canbeblocked_
    (:Block%20
      ;[0.15 0.15 0.15 0.5] OnBlock Calling
      (Default|CallOnBlocking Damage%20Causer)
      (return false))
    (:Damage
      ;[0.15 0.15 0.15 0.5] OnDamage Health Changes
      (bind _is_dead__ (CallFunction|DecreaseHealth _amount))
      (if _is_dead__
        ;[0.15 0.15 0.15 0.5] OnDeath
        (Variables|Health|SetIsDead%20? true)
        (Default|CallOnDeath)
        (return true)
        (else
          ;[0.15 0.15 0.15 0.5] OnDamage Call
          (if (or (Variables|State|GetIs%20Inturruptable) _shouldforceinturrupt)
            (Default|CallOnDamageResponse Damage%20Causer _damageresponse)
            (return true)))))
    (:No%20Damage
      (return false))))

(fn Healing
  (params (Percent :type Float%20%28double-precision%29))
  (bind _new_health (CallFunction|IncreaseHealth (* Percent (Variables|Health|GetMax%20Health))))
  (return _new_health))

(fn DecreaseHealth
  (params (Amount :type Float%20%28double-precision%29))
  (Variables|Health|SetHealth (Math|Float|Clamp(Float) (- (Variables|Health|GetHealth) Amount) 0.0 (Variables|Health|GetMax%20Health)))
  (Default|CallOnHealthUpdated (Variables|Health|GetHealth) (Variables|Health|GetMax%20Health))
  (return (<= (Variables|Health|GetHealth) 0.0)))

(fn IncreaseHealth
  (params (Amount :type Float%20%28double-precision%29))
  (bind _output_get (Variables|Health|SetHealth (Math|Float|Clamp(Float) (+ (Variables|Health|GetHealth) Amount) 0.0 (Variables|Health|GetMax%20Health))))
  (Default|CallOnHealthUpdated (Variables|Health|GetHealth) (Variables|Health|GetMax%20Health))
  (return _output_get))