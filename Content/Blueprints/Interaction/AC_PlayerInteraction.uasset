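; Player interaction component that lets the player trigger nearby actors implementing I_Interaction through press, hold or repeated-tap interactions.
; Collision overlaps maintain an array of candidates, with the last entry as the active target and state reset when one leaves.
; StartInteraction queries the target's type, then fires immediately, binds to a hold delegate until its duration elapses, or counts taps.
; A camera-forward trace endpoint helper is defined but unused in these graphs.
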(event Custom|OnBeginOverlap
  (params (OverlappedComponent :type Primitive%20Component%20Object%20Reference) (OtherActor :type Actor%20Object%20Reference) (OtherComp :type Primitive%20Component%20Object%20Reference) (OtherBodyIndex :type Integer) (bFromSweep :type Boolean) (SweepResult :type Hit%20Result%20Structure%20%28by%20ref%29))
  ;[0.15 0.15 0.15 0.5] OnBeginOverlap, Adding Actor to InteractiveActor Array if That Actor is Valid for Interaction.
  (if (Utilities|DoesObjectImplementInterface OtherActor "/Game/Blueprints/Interaction/I_Interaction.I_Interaction_C")
    (Utilities|Array|AddUnique (Variables|InteractiveActor|GetInteractive%20Actors) OtherActor)))

(event Custom|OnEndOverlap
  (params (OverlappedComponent :type Primitive%20Component%20Object%20Reference) (OtherActor :type Actor%20Object%20Reference) (OtherComp :type Primitive%20Component%20Object%20Reference) (OtherBodyIndex :type Integer))
  ;[0.15 0.15 0.15 0.5] OnEndingOverlap, Removing The Actor form InteractiveActors Array
  (if (Utilities|DoesObjectImplementInterface OtherActor "/Game/Blueprints/Interaction/I_Interaction.I_Interaction_C")
    (Utilities|Array|RemoveItem (Variables|InteractiveActor|GetInteractive%20Actors) OtherActor)
    (CallFunction|ResetInteractionState)))

(event Custom|StartInteraction
  ;[0.15 0.15 0.15 0.5] On Start Interactiong and assigning their unique InteractingType Logics
  ;;[0.15 0.15 0.15 0.5] Checking If there is any Interactive Actor, Then do Interacting Logic OR Else Dont Do anything
  (Utilities|IsValid (CallFunction|GETActiveInteractable)
    (:Is%20Valid
      ;;[0.15 0.15 0.15 0.5] GET Interact Type to Give difference interacting Logic as Per Type
      (bind _interacting_type (Class|IInteraction|CallGETInteractType(Message) (CallFunction|GETActiveInteractable)))
      (switch Utilities|FlowControl|Switch|SwitchonE_Interact_Type _interacting_type
        (:NewEnumerator0
          ;;[0.15 0.15 0.15 0.5] Press Logic - Direct Interact
          (CallFunction|ActualInteract))
        (:NewEnumerator1
          ;;[0.15 0.15 0.15 0.5] Hold Logic - Assigning OnInteractHold for Holding Logic
          (bind _duration (Class|IInteraction|CallGETHoldingDuration(Message) (CallFunction|GETActiveInteractable)))
          (Variables|Tracking|SetMax%20HoldDuration _duration)
          (EventDispatchers|BindEventtoOnHoldInteraction (EventDispatchers|CreateEvent :!event Custom|OnInteract%20Holding)))
        (:NewEnumerator2
          ;;[0.15 0.15 0.15 0.5] Tap Logic - Calling Direct Function for Taps
          (if (Variables|Tracking|GetIs%20ALR%20Get%20MaxCounts%20?)
            _
            (else
              (bind _counts (Class|IInteraction|CallGETTapCounts(Message) (CallFunction|GETActiveInteractable)))
              (Variables|Tracking|SetMax%20TapCounts%20 _counts)
              (Variables|Tracking|SetIs%20ALR%20Get%20MaxCounts%20? true)))
          (CallFunction|OnInteractTaps))))))

(event Custom|OnInteract%20Holding
  (params (Elapsed%20Seconds :type Float%20%28double-precision%29))
  ;[0.15 0.15 0.15 0.5] Holding Logic
  (if (>= Elapsed%20Seconds (Variables|Tracking|GetMax%20HoldDuration))
    (CallFunction|ActualInteract)
    (EventDispatchers|UnbindallEventsfromOnHoldInteraction)))

(event Custom|OnInteract%20Taps
  ;[0.15 0.15 0.15 0.5] Taps Logic
  (Variables|Tracking|SetCur%20Count (+ (Variables|Tracking|GetCur%20Count) (Variables|Tracking|GetCount%20One)))
  (if (<= (Variables|Tracking|GetMax%20TapCounts%20) (Variables|Tracking|GetCur%20Count))
    (CallFunction|ActualInteract)
    (Variables|Tracking|SetCur%20Count 0)
    (Variables|Tracking|SetMax%20TapCounts%20 0)
    (Variables|Tracking|SetIs%20ALR%20Get%20MaxCounts%20? false)))

(event Custom|ActualInteract
  ;[0.15 0.15 0.15 0.5] Actual Interact
  (Class|IInteraction|CallONInteractionBegin(Message) (CallFunction|GETActiveInteractable))
  (Variables|InteractiveActor|SetActive%20Interactable 0))

(event EventBeginPlay
  ;[0.15 0.15 0.15 0.5] BeginPlay
  (Utilities|FlowControl|Sequence
    (:then_0
      ;;[0.15 0.15 0.15 0.5] Cast to BP_Player
      (Utilities|Casting|CastToBP_Aurora_Player (Components|GetOwner)))
    (:then_1
      ;;[0.15 0.15 0.15 0.5] Setting The Collision Component. Then Binding Begin & End Overlap Event for Checking Interactive Actor in Range
      (Variables|Default|SetInteraction%20Collision (Variables|Default|GetInteractionCollision))
      (Collision|BindEventtoOnComponentBeginOverlap (Variables|Default|GetInteraction%20Collision) (EventDispatchers|CreateEvent :!event OnBeginOverlap))
      (Collision|BindEventtoOnComponentEndOverlap (Variables|Default|GetInteraction%20Collision) (EventDispatchers|CreateEvent :!event Custom|OnEndOverlap)))))

(fn GETActiveInteractable
  (bind _interactive_actors (Variables|InteractiveActor|GetInteractive%20Actors))
  (return (Utilities|Array|Get(acopy) _interactive_actors (Utilities|Array|LastIndex _interactive_actors))))

(fn ResetInteractionState
  (EventDispatchers|UnbindallEventsfromOnHoldInteraction)
  (Variables|Tracking|SetCur%20Count 0)
  (Variables|Tracking|SetIs%20ALR%20Get%20MaxCounts%20? false))

(fn TracingLenght
  (params (Range :type Float%20%28single-precision%29))
  (bind _followcamera (Variables|Default|GetFollowCamera))
  (bind _returnvalue (Transformation|GetWorldLocation _followcamera))
  (return _returnvalue (+ _returnvalue (* (Math|Vector|GetForwardVector _followcamera) Range))))