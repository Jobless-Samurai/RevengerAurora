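; BP_DummyTarget is a damageable target dummy actor that destroys itself when its damage component reports death.
; Health, max health, death state and damage handling are forwarded to the AC_Damagable component through wrapper functions.
; Healing is a stub that ignores its percent input and returns zero.
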(event OnDeath(AC_Damagable)
  (Actor|DestroyActor))

(fn ConstructionScript)

(fn GetCURHealth
  (return (Variables|/Game/Blueprints/Damage/AC_Damagable.AC_Damagable_C|GetHealth (Variables|Default|GetAC_Damagable))))

(fn GetMAXHealth
  (return (Variables|/Game/Blueprints/Damage/AC_Damagable.AC_Damagable_C|GetMax%20Health (Variables|Default|GetAC_Damagable))))

(fn Healing
  (params (Percent :type Float%20%28double-precision%29))
  (return 0.0))

(fn IsDead?
  (return (Variables|/Game/Blueprints/Damage/AC_Damagable.AC_Damagable_C|GetIsDead%20? (Variables|Default|GetAC_Damagable))))

(fn TakeDamage
  (params (Damage%20Info :type S%20Damage%20Info%20Structure) (Damage%20Causer :type Actor%20Object%20Reference))
  (bind _was_damaged__ (Default|TakeDamage (Variables|Default|GetAC_Damagable) Damage%20Info Damage%20Causer))
  (return _was_damaged__))